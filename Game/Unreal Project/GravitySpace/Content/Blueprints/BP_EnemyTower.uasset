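; Enemy tower obstacle that slides along Y on a timeline, firing bullets every second until destroyed, and removes itself when the movement finishes.
; Tick yaws the tower toward the player only while within a limited arc, and that same branch destroys it when game mode signals player death.
; Player bullet hits on "Destructable"-tagged components stop firing and tracking, destroy those components and the cannon, and consume the bullet.
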(event `self.ReceiveBeginPlay`
  (`|ExecutionSequence`
    (:`then_0`
      ;[1 1 1] Enemy Tower Shoot sequence
      (if (`self.NotDestroyed`) :!label _label
        (`|SpawnActorFromClass` "/Game/Blueprints/BP_EnemyBullet.BP_EnemyBullet_C" (`SceneComponent.K2_GetComponentToWorld` (`self.BulletSocket`)) "Undefined" "OverrideRootScale" null null)
        (`KismetSystemLibrary.Delay` 1.0)
        (goto _label)))
    (:`then_1`
      ;[1 1 1] Enemy Tower Movement
      (bind (_direction _position) (`Timeline|TowerMovement` :`NewTime` (`self.ObstacleVel`) :!via `PlayFromStart`)
        (:`Update`
          (`SceneComponent.K2_SetRelativeLocation` (`self.EnemyTower`) (`KismetMathLibrary.MakeVector` 0.0 _position) false false))
        (:`Finished`
          (`self.K2_DestroyActor`))))))

(event `self.ReceiveTick`
  (params (DeltaSeconds :type "Float (single-precision)"))
  (bind (_returnvalue_roll _returnvalue_pitch _returnvalue_yaw) (`KismetMathLibrary.BreakRotator` (`SceneComponent.K2_GetComponentRotation` (`self.TowerCollision`))))
  (bind (_returnvalue_roll_2 _returnvalue_pitch_2 _returnvalue_yaw_2) (`KismetMathLibrary.BreakRotator` (`KismetMathLibrary.FindLookAtRotation` (`SceneComponent.K2_GetComponentLocation` (`self.TowerCollision`)) (`SceneComponent.K2_GetComponentLocation` (`Actor.RootComponent` (`GameplayStatics.GetPlayerCharacter` 0))))))
  ;[1 1 1] Enemy Tower Rotation
  (if (`self.NotDestroyed`)
    (if (and (< _returnvalue_yaw 140.0) (> _returnvalue_yaw 40.0))
      (`SceneComponent.K2_SetWorldRotation` (`self.TowerCollision`) (`KismetMathLibrary.MakeRotator` 0.0 0.0 _returnvalue_yaw_2) false false)
      ;[1 1 1] Destroy after player death
      (bind _asbp_gravity_space_game_mode (cast `/Game/Blueprints/BP_GravitySpaceGameMode` (`GameplayStatics.GetGameMode`)))
      (if (== (`/Game/Blueprints/BP_GravitySpaceGameMode.GameMode` _asbp_gravity_space_game_mode) 2)
        (`self.K2_DestroyActor`)))))

(event `self.ReceiveHit`
  (params (MyComp :type "PrimitiveComponent Object Reference") (Other :type "Actor Object Reference") (OtherComp :type "PrimitiveComponent Object Reference") (bSelfMoved :type Boolean) (HitLocation :type "Vector Structure") (HitNormal :type "Vector Structure") (NormalImpulse :type "Vector Structure") (Hit :type "HitResult Structure (by ref)"))
  ;[1 1 1] Enemy Tower Collision
  (`self.DestroyOnShoot` MyComp Other MyComp Other))

(fn `DestroyOnShoot`
  (params (MyComponentTag :type "ActorComponent Object Reference") (AmmoTag :type "Actor Object Reference") (MyComponentToDestroy :type "PrimitiveComponent Object Reference") (OtherActorToDestroy :type "Actor Object Reference"))
  (bind _returnvalue (`self.ActorHasTag` AmmoTag "PlayerBullet"))
  (if (and (`ActorComponent.ComponentHasTag` MyComponentTag "Destructable") _returnvalue)
    (set `self.NotDestroyed` false)
    (`ActorComponent.K2_DestroyComponent` (`SceneComponent.GetChildrenComponents` MyComponentToDestroy true))
    (`ActorComponent.K2_DestroyComponent` MyComponentToDestroy)
    (`ActorComponent.K2_DestroyComponent` (`self.Cannon`)))
  (if _returnvalue
    (`self.K2_DestroyActor` OtherActorToDestroy)))

(fn `UserConstructionScript`)