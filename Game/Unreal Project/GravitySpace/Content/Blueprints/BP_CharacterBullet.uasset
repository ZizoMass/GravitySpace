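; BP_CharacterBullet is the player character's bullet actor, handling its own cleanup.
; Each tick it projects its collision component's world location to screen space and destroys itself when it passes above or below the viewport.
; While on screen, it checks BP_GravitySpaceGameMode and also destroys itself when GameMode equals 2, the player-death state.
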(event `self.ReceiveTick`
  (params (DeltaSeconds :type "Float (single-precision)"))
  (bind (_returnvalue_x _returnvalue_y) (`KismetMathLibrary.BreakVector2D` (`WidgetLayoutLibrary.GetViewportSize`)))
  (bind _screenlocation (`PlayerController.ProjectWorldLocationToScreen` (`GameplayStatics.GetPlayerController` 0) (`SceneComponent.K2_GetComponentLocation` (`self.BulletCollision`)) false))
  (if (or (< (`.Y` (`KismetMathLibrary.BreakVector2D` _screenlocation)) 0.0) (> (`.Y` (`KismetMathLibrary.BreakVector2D` _screenlocation)) _returnvalue_y))
    (`self.K2_DestroyActor`)
    (else
      ;[1 1 1] Destroy after player death
      (bind _asbp_gravity_space_game_mode (cast `/Game/Blueprints/BP_GravitySpaceGameMode` (`GameplayStatics.GetGameMode`)))
      (if (== (`/Game/Blueprints/BP_GravitySpaceGameMode.GameMode` _asbp_gravity_space_game_mode) 2)
        (`self.K2_DestroyActor`)))))

(fn `UserConstructionScript`)