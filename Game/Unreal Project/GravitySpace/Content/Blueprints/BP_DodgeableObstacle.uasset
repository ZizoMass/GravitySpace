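; Dodgeable two-block obstacle that moves through the level in the Gravity Space game, with a gap between the blocks.
; The Construction Script offsets the left and right blocks symmetrically on X by ObstacleGap.
; On BeginPlay, a timeline driven with ObstacleVel moves the Obstacles component along relative Y, then destroys the actor when finished.
; It destroys player bullets on hit and polls the game mode each Tick to remove itself after player death.
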(event `self.ReceiveHit`
  (params (MyComp :type "PrimitiveComponent Object Reference") (Other :type "Actor Object Reference") (OtherComp :type "PrimitiveComponent Object Reference") (bSelfMoved :type Boolean) (HitLocation :type "Vector Structure") (HitNormal :type "Vector Structure") (NormalImpulse :type "Vector Structure") (Hit :type "HitResult Structure (by ref)"))
  (if (`self.ActorHasTag` Other "PlayerBullet")
    (`self.K2_DestroyActor` Other)))

(event `self.ReceiveBeginPlay`
  ;[1 1 1] Move the Dodgeable Obstacle through the level
  (bind (_direction _objectycurve) (`Timeline|ObjectYMovement` :`NewTime` (`self.ObstacleVel`) :!via `PlayFromStart`)
    (:`Update`
      (`SceneComponent.K2_SetRelativeLocation` (`self.Obstacles`) (`KismetMathLibrary.MakeVector` 0.0 (.y _objectycurve)) false false))
    (:`Finished`
      (`self.K2_DestroyActor`))))

(event `self.ReceiveTick`
  (params (DeltaSeconds :type "Float (single-precision)"))
  ;[1 1 1] Destroy after player death
  (bind _asbp_gravity_space_game_mode (cast `/Game/Blueprints/BP_GravitySpaceGameMode` (`GameplayStatics.GetGameMode`)))
  (if (== (`/Game/Blueprints/BP_GravitySpaceGameMode.GameMode` _asbp_gravity_space_game_mode) 2)
    (`self.K2_DestroyActor`)))

(fn `UserConstructionScript`
  (bind _obstaclegap (`self.ObstacleGap`))
  (`SceneComponent.K2_SetRelativeLocation` (`self.BlockLeft`) (`KismetMathLibrary.MakeVector` _obstaclegap) false false)
  (`SceneComponent.K2_SetRelativeLocation` (`self.BlockRight`) (`KismetMathLibrary.MakeVector` (* _obstaclegap -1.0)) false false))