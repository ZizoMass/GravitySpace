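; BP_EnemyBullet is an enemy projectile that player bullets can shoot down, with its sprite tinted red at construction.
; On Hit, DestroyOnShoot destroys both actors if the other is tagged PlayerBullet, first removing the struck component if tagged Destructable.
; Each Tick, it projects the collision component to screen space and destroys itself once above or below the viewport.
; It contains no player damage or movement logic.
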(event `self.ReceiveHit`
  (params (MyComp :type "PrimitiveComponent Object Reference") (Other :type "Actor Object Reference") (OtherComp :type "PrimitiveComponent Object Reference") (bSelfMoved :type Boolean) (HitLocation :type "Vector Structure") (HitNormal :type "Vector Structure") (NormalImpulse :type "Vector Structure") (Hit :type "HitResult Structure (by ref)"))
  (`self.DestroyOnShoot` MyComp Other MyComp Other))

(event `self.ReceiveTick`
  (params (DeltaSeconds :type "Float (single-precision)"))
  (bind (_returnvalue_x _returnvalue_y) (`KismetMathLibrary.BreakVector2D` (`WidgetLayoutLibrary.GetViewportSize`)))
  (bind _screenlocation (`PlayerController.ProjectWorldLocationToScreen` (`GameplayStatics.GetPlayerController` 0) (`SceneComponent.K2_GetComponentLocation` (`self.BulletCollision`)) false))
  (if (or (< (`.Y` (`KismetMathLibrary.BreakVector2D` _screenlocation)) 0.0) (> (`.Y` (`KismetMathLibrary.BreakVector2D` _screenlocation)) _returnvalue_y))
    (`self.K2_DestroyActor`)))

(fn `DestroyOnShoot`
  (params (MyComponentTag :type "ActorComponent Object Reference") (AmmoTag :type "Actor Object Reference") (MyComponentToDestroy :type "PrimitiveComponent Object Reference") (OtherActorToDestroy :type "Actor Object Reference"))
  (bind _returnvalue (`self.ActorHasTag` AmmoTag "PlayerBullet"))
  (if (and (`ActorComponent.ComponentHasTag` MyComponentTag "Destructable") _returnvalue)
    (`ActorComponent.K2_DestroyComponent` MyComponentToDestroy))
  (if _returnvalue
    (`self.K2_DestroyActor` OtherActorToDestroy)
    (`self.K2_DestroyActor`)))

(fn `UserConstructionScript`
  (`PaperFlipbookComponent.SetSpriteColor` (`self.PF_SpaceshipBullet`) (struct :`R` 1.0 :`G` 0.028286 :`A` 1.0)))