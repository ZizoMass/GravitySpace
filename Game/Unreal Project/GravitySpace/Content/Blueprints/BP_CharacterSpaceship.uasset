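; Player spaceship Character that auto-fires bullets while fighting a horizontal gravity field.
; After a random first nudge, Tick launches it by X offset times GravityIntensity; holding touch or Propel charges a timeline-driven counter-launch toward center, fired on release or completion.
; Arrows show the propel direction.
; Enemy or obstacle overlaps and wing sensors leaving the screen trigger destruction, which hides and resets the ship, saves the high score and switches GameMode state.
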(event `self.CapsuleComponent.OnComponentBeginOverlap`
  (params (OverlappedComponent :type "PrimitiveComponent Object Reference") (OtherActor :type "Actor Object Reference") (OtherComp :type "PrimitiveComponent Object Reference") (OtherBodyIndex :type Integer) (bFromSweep :type Boolean) (SweepResult :type "HitResult Structure (by ref)"))
  ;[1 1 1] Collision Detection
  (if (`self.ActorHasTag` OtherActor "EnemySpaceship")
    (if (`self.ActorHasTag` OtherActor "Destructable")
      (`self.K2_DestroyActor` (stale `self.Box.OnComponentBeginOverlap` OtherActor) :!label _label)
      (`self.K2_DestroyActor` OtherActor))
    (`self.PlayerSpaceshipDestroyed` :!label _label_2)))

(event `self.Box.OnComponentBeginOverlap`
  (params (OverlappedComponent :type "PrimitiveComponent Object Reference") (OtherActor :type "Actor Object Reference") (OtherComp :type "PrimitiveComponent Object Reference") (OtherBodyIndex :type Integer) (bFromSweep :type Boolean) (SweepResult :type "HitResult Structure (by ref)"))
  ;[1 1 1] Collision Detection
  (`KismetSystemLibrary.PrintString` "Hello")
  (if (or (`self.ActorHasTag` OtherActor "Obstacle") (`ActorComponent.ComponentHasTag` OtherComp "Obstacle"))
    (if (`self.ActorHasTag` OtherActor "Destructable")
      (goto _label)
      (else
        (goto _label_2)))))

(event `GameStart`
  ;[1 1 1] Apply First Pull on Spaceship
  (`KismetSystemLibrary.Delay` 0.2)
  (`SceneComponent.SetHiddenInGame` (`self.Mesh`) false true)
  (`ActorComponent.Activate` (`self.CharacterMovement`) true)
  (`|MultiGate` true true
    (:`Out 0`
      (`self.LaunchCharacter` (-50.0 0.0 0.0)))
    (:`Out 1`
      (`self.LaunchCharacter` (50.0 0.0 0.0))))
  ;[1 1 1] Spaceship auto shoot
  (bind _asbp_gravity_space_game_mode (cast `/Game/Blueprints/BP_GravitySpaceGameMode` (`GameplayStatics.GetGameMode`)))
  (`KismetSystemLibrary.Delay` (`self.ShootSpawnVel`) :!label _label_3)
  (if (== (`/Game/Blueprints/BP_GravitySpaceGameMode.GameMode` _asbp_gravity_space_game_mode) 1)
    (bind _returnvalue (`|SpawnActorFromClass` "/Game/Blueprints/BP_CharacterBullet.BP_CharacterBullet_C" (`KismetMathLibrary.MakeTransform` (`SceneComponent.GetSocketLocation` (`self.Mesh`) "Ammo")) "AlwaysSpawn" "OverrideRootScale" null null))
    (`self.K2_DetachFromActor` _returnvalue "KeepRelative" "KeepRelative" "KeepRelative")
    (goto _label_3)))

(event `self.ReceiveTick`
  (params (DeltaSeconds :type "Float (single-precision)"))
  (bind _returnvalue_x (`KismetMathLibrary.BreakVector2D` (`WidgetLayoutLibrary.GetViewportSize`)))
  (bind _returnvalue_x_2 (`KismetMathLibrary.BreakVector2D` (`WidgetLayoutLibrary.GetViewportSize`)))
  (bind _screenlocation (`PlayerController.ProjectWorldLocationToScreen` (`GameplayStatics.GetPlayerController` 0) (`SceneComponent.K2_GetComponentLocation` (`self.LeftWing`)) false))
  (bind _screenlocation_2 (`PlayerController.ProjectWorldLocationToScreen` (`GameplayStatics.GetPlayerController` 0) (`SceneComponent.K2_GetComponentLocation` (`self.RightWing`)) false))
  ;[1 1 1] Gravity field
  (`self.LaunchCharacter` (`KismetMathLibrary.MakeVector` (* (.x (.location (`self.GetTransform`))) (`self.GravityIntensity`))))
  (`self.ReferenceArrows`)
  ;[1 1 1] If the spaceship touches the edges, it moves it back to the center of the screen and stops its movements for a while
  (if (or (or (< (`KismetMathLibrary.BreakVector2D` _screenlocation_2) 0.0) (> (`KismetMathLibrary.BreakVector2D` _screenlocation_2) _returnvalue_x_2)) (or (< (`KismetMathLibrary.BreakVector2D` _screenlocation) 0.0) (> (`KismetMathLibrary.BreakVector2D` _screenlocation) _returnvalue_x)))
    (`self.PlayerSpaceshipDestroyed`)))

(event `InputTouch` :consume false
  (params (Location :type "Vector Structure") (FingerIndex :type "ETouchIndex Enum"))
  (bind _propelstrengh (`self.PropelStrengh`))
  ;[1 1 1] Player Spaceship Control
  (:`Pressed`
    (if (< (.x (.location (`self.GetTransform`))) 0.0) :!label _label_4
      (set `self.ChargingRight` true)
      (bind (_direction _propelvelocityright) (`Timeline|PropelVelocityCharge_Right` :!via `PlayFromStart` :!label _label_5)
        (:`Update`
          (bind _output_get (set `self.PropelCharge` _propelvelocityright)))
        (:`Finished`
          (set `self.PropelRelease` true)
          (if (`self.PropelRelease`) :!label _label_6
            (bind _returnvalue (* _output_get _propelstrengh))
            (`self.LaunchCharacter` (`KismetMathLibrary.MakeVector` _returnvalue) true true)
            (`KismetSystemLibrary.PrintString` (`KismetStringLibrary.Conv_DoubleToString` _returnvalue) false false)
            (set `self.PropelRelease` false :!label _label_7))))
      (else
        (set `self.ChargingRight` false)
        (bind (_direction_2 _propelvelocityleft) (`Timeline|PropelVelocityCharge_Left` :!via `PlayFromStart` :!label _label_8)
          (:`Update`
            (bind _output_get_2 (set `self.PropelCharge` _propelvelocityleft)))
          (:`Finished`
            (set `self.PropelRelease` true :!label _label_9)
            (if (`self.PropelRelease`)
              (bind _returnvalue_2 (* _output_get_2 _propelstrengh))
              (`self.LaunchCharacter` (`KismetMathLibrary.MakeVector` _returnvalue_2) true true)
              (`KismetSystemLibrary.PrintString` (`KismetStringLibrary.Conv_DoubleToString` _returnvalue_2) false false)
              (goto _label_7)))))))
  (:`Released`
    (set `self.PropelRelease` true :!label _label_10)
    (if (`self.ChargingRight`)
      (`|ExecutionSequence`
        (:`then_0`
          (goto _label_5 :!via `Stop`))
        (:`then_1`
          (goto _label_6)))
      (else
        (`|ExecutionSequence`
          (:`then_0`
            (goto _label_8 :!via `Stop`))
          (:`then_1`
            (goto _label_9)))))))

(event `InputAction|Propel`
  (params (Key :type "Key Structure"))
  ;[1 1 1] Player Spaceship Control
  (:`Pressed`
    (goto _label_4))
  (:`Released`
    (goto _label_10)))

(fn `PlayerSpaceshipDestroyed`
  (`SceneComponent.SetHiddenInGame` (`self.Mesh`) true true)
  (`self.K2_SetActorTransform` (`self.SpaceshipStartLocation`))
  (`ActorComponent.Deactivate` (`self.CharacterMovement`))
  (bind _asbp_game_instance (cast `/Game/Blueprints/BP_GameInstance` (`GameplayStatics.GetGameInstance`)))
  (`/Game/Blueprints/BP_GameInstance.SetPlayerHighScore` _asbp_game_instance)
  (bind _asbp_gravity_space_game_mode (cast `/Game/Blueprints/BP_GravitySpaceGameMode` (`GameplayStatics.GetGameMode`)))
  (set `/Game/Blueprints/BP_GravitySpaceGameMode.GameMode` 2 _asbp_gravity_space_game_mode))

(fn `ReferenceArrows`
  (bind _jumpleft (`self.JumpLeft`))
  (bind _jumpright (`self.JumpRight`))
  (bind _asbp_gravity_space_game_mode (cast `/Game/Blueprints/BP_GravitySpaceGameMode` (`GameplayStatics.GetGameMode`)))
  (if (== (`/Game/Blueprints/BP_GravitySpaceGameMode.GameMode` _asbp_gravity_space_game_mode) 1)
    (if (< (.x (.location (`self.GetTransform`))) 0.0)
      (`SceneComponent.SetVisibility` _jumpleft false false)
      (`SceneComponent.SetVisibility` _jumpright true false)
      (else
        (`SceneComponent.SetVisibility` _jumpleft true false)
        (`SceneComponent.SetVisibility` _jumpright false false)))))

(fn `UserConstructionScript`
  (bind _lateraldetection (`self.LateralDetection`))
  ;[1 1 1] Defines the distance at which the side sensors are.
  (`SceneComponent.K2_SetRelativeTransform` (`self.RightWing`) (`KismetMathLibrary.MakeTransform` (`KismetMathLibrary.MakeVector` _lateraldetection)) false false)
  (`SceneComponent.K2_SetRelativeTransform` (`self.LeftWing`) (`KismetMathLibrary.MakeTransform` (`KismetMathLibrary.MakeVector` (* _lateraldetection -1.0))) false false)
  ;[1 1 1] Set Player Start Location
  (set `self.SpaceshipStartLocation` (`self.GetTransform`)))