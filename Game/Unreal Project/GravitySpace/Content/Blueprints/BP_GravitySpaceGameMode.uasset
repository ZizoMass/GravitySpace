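; BP_GravitySpaceGameMode is the game mode that switches the game's UI between main menu, playing and game-over states.
; Every Tick it switches on the GameMode variable, clears all widgets and creates that state's widget afresh, rather than only on state changes.
; The menu state also unhides the player spaceship mesh, while the playing state increments PlayerScore in BP_GameInstance each frame, so score grows with frames survived.
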(event `self.ReceiveTick`
  (params (DeltaSeconds :type "Float (single-precision)"))
  (switch `int` (`self.GameMode`)
    (:`0`
      (`WidgetLayoutLibrary.RemoveAllWidgets`)
      (bind _returnvalue (`|CreateWidget` "/Game/UI/Widgets/WB_GameMainMenu.WB_GameMainMenu_C" (`GameplayStatics.GetPlayerController` 0)))
      (bind _output_get (set `self.MainMenuWidget` _returnvalue))
      (`UserWidget.AddToViewport` _output_get 0)
      (bind _asbp_character_spaceship (cast `/Game/Blueprints/BP_CharacterSpaceship` (`GameplayStatics.GetPlayerCharacter` 0)))
      (`SceneComponent.SetHiddenInGame` (`Character.Mesh` _asbp_character_spaceship) false true))
    (:`1`
      (`WidgetLayoutLibrary.RemoveAllWidgets`)
      (bind _returnvalue_2 (`|CreateWidget` "/Game/UI/Widgets/WB_PlayerScoreHUD.WB_PlayerScoreHUD_C" (`GameplayStatics.GetPlayerController` 0)))
      (`UserWidget.AddToViewport` _returnvalue_2 0)
      (bind _asbp_game_instance (cast `/Game/Blueprints/BP_GameInstance` (`GameplayStatics.GetGameInstance`)))
      (set `/Game/Blueprints/BP_GameInstance.PlayerScore` (+ (`/Game/Blueprints/BP_GameInstance.PlayerScore` _asbp_game_instance) 1) _asbp_game_instance))
    (:`2`
      (`WidgetLayoutLibrary.RemoveAllWidgets`)
      (bind _returnvalue_3 (`|CreateWidget` "/Game/UI/Widgets/WB_GameOver.WB_GameOver_C" (`GameplayStatics.GetPlayerController` 0)))
      (`UserWidget.AddToViewport` _returnvalue_3 0))))

(fn `UserConstructionScript`)