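; Enemy spaceship that flies a timeline-driven path, fires bullets and destroys itself when the path ends.
; BeginPlay randomly picks a direction that mirrors the path's X offset on the Box component.
; Timeline events open and close a gate around a delayed loop spawning BP_EnemyBullet at BulletSocket.
; A Box hit tagged PlayerBullet destroys both actors, and Tick polls the game mode to remove the ship after player death.
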(event `self.ReceiveBeginPlay`
  ;[1 1 1] Enemy spaceship movement
  (`|MultiGate` true
    (:`Out 0`
      (set `self.SpaceshipDirection` 1.0)
      (bind (_direction _newtrack_0) (`Timeline|SpaceshipMovement` :!via `PlayFromStart` :!label _label)
        (:`Update`
          (`SceneComponent.K2_SetRelativeLocation` (`self.Box`) (`KismetMathLibrary.MakeVector` (* (.x _newtrack_0) (`self.SpaceshipDirection`)) (.y _newtrack_0)) false false))
        (:`Finished`
          (`self.K2_DestroyActor`))
        (:`StartShoot`
          ;[1 1 1] Enemy Spaceship shot sequence
          (`/Engine/EditorBlueprintResources/StandardMacros.Gate` false :!label _label_2
            (:`Exit`
              (`|SpawnActorFromClass` "/Game/Blueprints/BP_EnemyBullet.BP_EnemyBullet_C" (`SceneComponent.K2_GetComponentToWorld` (`self.BulletSocket`)) "Undefined" "OverrideRootScale" null null)
              (`KismetSystemLibrary.Delay` 0.5)
              (goto _label_2))))
        (:`StoopShoot`
          (goto _label_2 :!via `Close`))))
    (:`Out 1`
      (set `self.SpaceshipDirection` -1.0)
      (goto _label :!via `PlayFromStart`))))

(event `self.Box.OnComponentHit`
  (params (HitComponent :type "PrimitiveComponent Object Reference") (OtherActor :type "Actor Object Reference") (OtherComp :type "PrimitiveComponent Object Reference") (NormalImpulse :type "Vector Structure") (Hit :type "HitResult Structure (by ref)"))
  ;[1 1 1] Enemy Spaceship hit detection
  (if (`self.ActorHasTag` OtherActor "PlayerBullet")
    (`self.K2_DestroyActor` OtherActor)
    (`self.K2_DestroyActor`)))

(event `self.ReceiveTick`
  (params (DeltaSeconds :type "Float (single-precision)"))
  ;[1 1 1] Destroy after player death
  (bind _asbp_gravity_space_game_mode (cast `/Game/Blueprints/BP_GravitySpaceGameMode` (`GameplayStatics.GetGameMode`)))
  (if (== (`/Game/Blueprints/BP_GravitySpaceGameMode.GameMode` _asbp_gravity_space_game_mode) 2)
    (`self.K2_DestroyActor`)))

(fn `DestroyOnShoot`
  (params (MyComponentTag :type "ActorComponent Object Reference") (AmmoTag :type "Actor Object Reference") (MyComponentToDestroy :type "PrimitiveComponent Object Reference") (OtherActorToDestroy :type "Actor Object Reference")))

(fn `UserConstructionScript`)