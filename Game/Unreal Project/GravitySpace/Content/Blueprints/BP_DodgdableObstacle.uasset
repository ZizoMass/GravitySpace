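; Dodgeable obstacle actor made of a left and right block separated by a configurable gap, which travels through the level.
; The construction script places the two blocks symmetrically along X using ObstacleGap.
; On BeginPlay, a latent MoveComponentTo slides the Obstacles component along relative Y, then the actor destroys itself.
; ObstacleVel feeds the move's OverTime, so it acts as a travel duration rather than a speed.
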(event `self.ReceiveBeginPlay`
  ;[1 1 1] Move the Dodgeable Obstacle through the level
  (`KismetSystemLibrary.MoveComponentTo` (`self.Obstacles`) (0.0 8000.0 0.0) (struct) false false (`self.ObstacleVel`))
  (`self.K2_DestroyActor`))

(fn `UserConstructionScript`
  (bind _obstaclegap (`self.ObstacleGap`))
  (`SceneComponent.K2_SetRelativeLocation` (`self.BlockLeft`) (`KismetMathLibrary.MakeVector` _obstaclegap) false false)
  (`SceneComponent.K2_SetRelativeLocation` (`self.BlockRight`) (`KismetMathLibrary.MakeVector` (* _obstaclegap -1.0)) false false))