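; Dodgeable obstacle for a gravity space game: two side blocks with a shootable block filling the gap between them.
; The construction script positions the side blocks and scales the middle block from ObstacleGap.
; A timeline moves the obstacle along Y, then destroys the actor; Tick also destroys it when the game mode signals player death.
; Player bullets are destroyed on hit and remove only components tagged "Destructable".
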(event `self.ReceiveHit`
  (params (MyComp :type "PrimitiveComponent Object Reference") (Other :type "Actor Object Reference") (OtherComp :type "PrimitiveComponent Object Reference") (bSelfMoved :type Boolean) (HitLocation :type "Vector Structure") (HitNormal :type "Vector Structure") (NormalImpulse :type "Vector Structure") (Hit :type "HitResult Structure (by ref)"))
  (`self.DestroyOnShoot` MyComp Other MyComp Other))

(event `self.ReceiveBeginPlay`
  ;[1 1 1] Move the Dodgeable Obstacle through the level
  (bind (_direction _ymovementcurve) (`Timeline|ObjectYMovement` :`NewTime` (`self.ObstacleVel`) :!via `PlayFromStart`)
    (:`Update`
      (`SceneComponent.K2_SetRelativeLocation` (`self.Obstacles`) (`KismetMathLibrary.MakeVector` 0.0 (. _ymovementcurve)) false false))
    (:`Finished`
      (`self.K2_DestroyActor`))))

(event `self.ReceiveTick`
  (params (DeltaSeconds :type "Float (single-precision)"))
  ;[1 1 1] Destroy after player death
  (bind _asbp_gravity_space_game_mode (cast `/Game/Blueprints/BP_GravitySpaceGameMode` (`GameplayStatics.GetGameMode`)))
  (if (== (`/Game/Blueprints/BP_GravitySpaceGameMode.GameMode` _asbp_gravity_space_game_mode) 2)
    (`self.K2_DestroyActor`)))

(fn `DestroyOnShoot`
  (params (MyComponentTag :type "ActorComponent Object Reference") (AmmoTag :type "Actor Object Reference") (MyComponentToDestroy :type "PrimitiveComponent Object Reference") (OtherActorToDestroy :type "Actor Object Reference"))
  (bind _returnvalue (`self.ActorHasTag` AmmoTag "PlayerBullet"))
  (if (and (`ActorComponent.ComponentHasTag` MyComponentTag "Destructable") _returnvalue)
    (`ActorComponent.K2_DestroyComponent` MyComponentToDestroy))
  (if _returnvalue
    (`self.K2_DestroyActor` OtherActorToDestroy)))

(fn `UserConstructionScript`
  (bind _obstaclegap (`self.ObstacleGap`))
  (`SceneComponent.K2_SetRelativeLocation` (`self.BlockLeft`) (`KismetMathLibrary.MakeVector` _obstaclegap) false false)
  (`SceneComponent.K2_SetRelativeLocation` (`self.BlockRight`) (`KismetMathLibrary.MakeVector` (* _obstaclegap -1.0)) false false)
  (`SceneComponent.SetRelativeScale3D` (`self.DestructibleBlock`) (`KismetMathLibrary.MakeVector` (/ _obstaclegap 150.0) 1.0 2.0)))